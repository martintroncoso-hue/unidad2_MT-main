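; BP_Npc2 is an NPC Blueprint that shows a multi-line dialogue on screen when interacted with.
; Each Interact event creates a WB_Dialogo widget if none exists, writes the current Dialogo entry into its text and advances the index.
; Once every line has been shown, the next interaction removes the widget and resets the index so the dialogue can replay.
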(event EventBeginPlay)

(event Collision|EventActorBeginOverlap
  (params (OtherActor :type Actor%20Object%20Reference)))

(event EventTick
  (params (DeltaSeconds :type Float%20%28single-precision%29)))

(event EventInteract
  (if (< (Variables|Default|GetDialogo%20index) (Utilities|Array|Length (Variables|Default|GetDialogo)))
    (Variables|Default|GetDialogoRef
      (:then
        _)
      (:else
        (bind _returnvalue (UserInterface|CreateWidget "/Game/BP/WB_Dialogo.WB_Dialogo_C" (Game|GetPlayerController 0)))
        (bind _output_get (Variables|Default|SetDialogoRef _returnvalue))
        (UserInterface|Viewport|AddtoViewport _output_get 0)))
    (Rendering|Components|TextRender|SetText (Variables|/Game/BP/WB_Dialogo.WB_Dialogo_C|GetDialogo_01 (Variables|Default|GetDialogoRef)) (Utilities|Text|ToText(String) (Utilities|Array|Get(acopy) (Variables|Default|GetDialogo) (Variables|Default|GetDialogo%20index))))
    (Math|Integer|IncrementInt (Variables|Default|GetDialogo%20index))
    (else
      (Widget|RemovefromParent (Variables|Default|GetDialogoRef))
      (Variables|Default|SetDialogoRef 0)
      (Variables|Default|SetDialogo%20index 0))))

(fn ConstructionScript)